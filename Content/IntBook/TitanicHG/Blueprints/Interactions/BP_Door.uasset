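; BP_Door is an interactable door that highlights when looked at and rotates open or closed on interact.
; Look events toggle custom depth stencil outlining and drive a looping timeline that blinks material color.
; When looking ends, the blink finishes forward or reverses based on elapsed time.
; A FlipFlop plays or reverses the 90-degree rotation timeline, whose finish direction sets IsDoorOpen.
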(event EventInputInteractPressed
  (params (NewParam :type Key%20Structure))
  (bind _door (Variables|Default|GetDoor))
  ;[1 1 1] Door Animation
  (Utilities|FlowControl|FlipFlop
    (:A
      (bind (_direction _doorrotation) (Timeline|DoorAnimation Play)
        (:Update
          (Components|MoveComponentTo _door (Variables|/Script/Engine.SceneComponent|GetRelativeLocation _door) (Math|Rotator|Lerp(Rotator) "0, 0, 0" "0,90.000000, 0" _doorrotation true) false false 0.0 false))
        (:Finished
          (switch Utilities|FlowControl|Switch|SwitchonETimelineDirection _direction
            (:Forward
              (Variables|Default|SetIsDoorOpen true))
            (:Backward
              (Variables|Default|SetIsDoorOpen false))))))
    (:B
      (Timeline|DoorAnimation Reverse))))

(event EventBeginLookingat
  ;[1 1 1] Set RenderDepth Outline
  (Rendering|SetRenderCustomDepth (Variables|Default|GetDoor) true)
  (Rendering|SetCustomDepthStencilValue (Variables|Default|GetDoor) 2)
  (Components|Timeline|SetLooping (Variables|Default|GetBlinkColorTimeline) true)
  (Components|Timeline|SetPlayRate (Variables|Default|GetBlinkColorTimeline) (Variables|Default|GetBlinkSpeed))
  (bind (_direction _color _time) (Timeline|BlinkColorTimeline Play)
    (:Update
      (Variables|Default|SetTime _time)
      (Rendering|Material|SetVectorParameterValueonMaterials (Variables|Default|GetDoor) "BlinkColor" (Math|Conversions|ToVector(LinearColor) _color))
      (Rendering|Material|SetScalarParameterValueonMaterials (Variables|Default|GetDoor) "BlinkIntensity" (Variables|Default|GetBlinkIntensity)))))

(event EventEndLookingat
  ;[1 1 1] Set RenderDepth Outline
  (Rendering|SetRenderCustomDepth (Variables|Default|GetDoor) false)
  (Rendering|SetCustomDepthStencilValue (Variables|Default|GetDoor) 0)
  (Components|Timeline|SetLooping (Variables|Default|GetBlinkColorTimeline) false)
  (Components|Timeline|SetPlayRate (Variables|Default|GetBlinkColorTimeline) (* (Variables|Default|GetBlinkSpeed) 1.0))
  (if (>= (Variables|Default|GetTime) 0.75)
    (bind (_direction _color _time) (Timeline|BlinkColorTimeline Play)
      (:Update
        (Variables|Default|SetTime _time)
        (Rendering|Material|SetVectorParameterValueonMaterials (Variables|Default|GetDoor) "BlinkColor" (Math|Conversions|ToVector(LinearColor) _color))
        (Rendering|Material|SetScalarParameterValueonMaterials (Variables|Default|GetDoor) "BlinkIntensity" (Variables|Default|GetBlinkIntensity))))
    (else
      (Timeline|BlinkColorTimeline Reverse))))

(fn ConstructionScript)