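; Testimonial card actor that the player can highlight, pick up, read, flip and dismiss.
; Looking at or cursor-hovering it drives a custom-depth outline and blinking material timeline while interaction is allowed.
; Interacting attaches the card to the player, animates it forward with depth-of-field and fades in a testimonial widget.
; Flip alternates a rotation timeline; interacting once fully shown restores player control, spawns a particle component and destroys the actor.
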(event EventBeginCursorOverlap
  ;[1 1 1] Set RenderDepth Outline
  (bind _asbp_player_character_01 (Utilities|Casting|CastToBP_PlayerCharacter_01 (Game|GetPlayerCharacter 0)))
  (bind _output_get (Variables|Default|SetAs%20BP%20Player%20Character%2001 _asbp_player_character_01))
  (if (Variables|/Game/IntBook/TitanicHG/Characters/Player/PlayerCharacter_01/BP_PlayerCharacter_01.BP_PlayerCharacter_01_C|GetCanInteract _output_get)
    (Rendering|SetRenderCustomDepth (Variables|Default|GetTestimonialCard) true)
    (Rendering|SetCustomDepthStencilValue (Variables|Default|GetTestimonialCard) 2)
    (Components|Timeline|SetLooping (Variables|Default|GetBlinkColorTimeline) true)
    (Components|Timeline|SetPlayRate (Variables|Default|GetBlinkColorTimeline) (Variables|Default|GetBlinkSpeed))
    (bind (_direction _color _time) (Timeline|BlinkColorTimeline Play)
      (:Update
        (Variables|Default|SetTime _time)
        (Rendering|Material|SetVectorParameterValueonMaterials (Variables|Default|GetTestimonialCard) "BlinkColor" (Math|Conversions|ToVector(LinearColor) _color))
        (Rendering|Material|SetScalarParameterValueonMaterials (Variables|Default|GetTestimonialCard) "BlinkIntensity" (Variables|Default|GetBlinkIntensity))))
    (else
      (Rendering|SetRenderCustomDepth (Variables|Default|GetTestimonialCard) false)
      (Rendering|SetCustomDepthStencilValue (Variables|Default|GetTestimonialCard) 0)
      (Components|Timeline|SetLooping (Variables|Default|GetBlinkColorTimeline) false)
      (Components|Timeline|SetPlayRate (Variables|Default|GetBlinkColorTimeline) (* (Variables|Default|GetBlinkSpeed) 1.0))
      (if (>= (Variables|Default|GetTime) 0.75)
        (Timeline|BlinkColorTimeline Play)
        (else
          (Timeline|BlinkColorTimeline Reverse))))))

(event EventEndCursorOverlap
  ;[1 1 1] Set RenderDepth Outline
  (Rendering|SetRenderCustomDepth (Variables|Default|GetTestimonialCard) false)
  (Rendering|SetCustomDepthStencilValue (Variables|Default|GetTestimonialCard) 0)
  (Components|Timeline|SetLooping (Variables|Default|GetBlinkColorTimeline) false)
  (Components|Timeline|SetPlayRate (Variables|Default|GetBlinkColorTimeline) (* (Variables|Default|GetBlinkSpeed) 1.0))
  (if (>= (Variables|Default|GetTime) 0.75)
    (bind (_direction _color _time) (Timeline|BlinkColorTimeline Play)
      (:Update
        (Variables|Default|SetTime _time)
        (Rendering|Material|SetVectorParameterValueonMaterials (Variables|Default|GetTestimonialCard) "BlinkColor" (Math|Conversions|ToVector(LinearColor) _color))
        (Rendering|Material|SetScalarParameterValueonMaterials (Variables|Default|GetTestimonialCard) "BlinkIntensity" (Variables|Default|GetBlinkIntensity))))
    (else
      (Timeline|BlinkColorTimeline Reverse))))

(event EventInputInteractPressed
  (params (NewParam :type Key%20Structure))
  (bind _as_bp_player_character_01 (Variables|Default|GetAs%20BP%20Player%20Character%2001))
  (bind _as_bp_player_character_01_2 (Variables|Default|GetAs%20BP%20Player%20Character%2001))
  (bind _as_bp_player_character_01_3 (Variables|Default|GetAs%20BP%20Player%20Character%2001))
  (bind _as_bp_player_character_01_4 (Variables|Default|GetAs%20BP%20Player%20Character%2001))
  (bind _as_bp_player_character_01_5 (Variables|Default|GetAs%20BP%20Player%20Character%2001))
  ;[1 1 1] Card Animation
  (Utilities|FlowControl|Sequence
    (:then_0
      (if (not (Variables|Default|GetFullyRendered))
        (Class|InterfaceObjectInteraction|DisableCursor(Message) _as_bp_player_character_01_5)
        (if (Math|Boolean|ANDBoolean (Variables|/Game/IntBook/TitanicHG/Characters/Player/PlayerCharacter_01/BP_PlayerCharacter_01.BP_PlayerCharacter_01_C|GetCanInteract _as_bp_player_character_01_5) (Variables|/Game/IntBook/TitanicHG/Characters/Player/PlayerCharacter_01/BP_PlayerCharacter_01.BP_PlayerCharacter_01_C|GetCanPickUp _as_bp_player_character_01_5) (not (Variables|/Game/IntBook/TitanicHG/Characters/Player/PlayerCharacter_01/BP_PlayerCharacter_01.BP_PlayerCharacter_01_C|GetAmInteracting _as_bp_player_character_01_5)))
          (Variables|/Game/IntBook/TitanicHG/Characters/Player/PlayerCharacter_01/BP_PlayerCharacter_01.BP_PlayerCharacter_01_C|SetCanEnableMouse _as_bp_player_character_01_3 false)
          (Variables|/Game/IntBook/TitanicHG/Characters/Player/PlayerCharacter_01/BP_PlayerCharacter_01.BP_PlayerCharacter_01_C|SetAmInteracting _as_bp_player_character_01_3 true)
          (Variables|/Game/IntBook/TitanicHG/Characters/Player/PlayerCharacter_01/BP_PlayerCharacter_01.BP_PlayerCharacter_01_C|SetObjectInteractingWith _as_bp_player_character_01_3 self)
          (Variables|/Game/IntBook/TitanicHG/Characters/Player/PlayerCharacter_01/BP_PlayerCharacter_01.BP_PlayerCharacter_01_C|SetCanInteract _as_bp_player_character_01_3 false)
          (Class|InterfaceObjectInteraction|DisableMovement(Message) _as_bp_player_character_01)
          (Transformation|AttachComponentToComponent (Variables|Default|GetTestimonialCard) (Variables|/Game/IntBook/TitanicHG/Characters/Player/PlayerCharacter_01/BP_PlayerCharacter_01.BP_PlayerCharacter_01_C|GetCardComponent _as_bp_player_character_01) "None" "KeepWorld" "KeepWorld" "KeepRelative" true)
          (bind _output_get (Variables|Default|SetInitialLocation (Transformation|GetRelativeTransform (Variables|Default|GetTestimonialCard))))
          (bind (_direction _pickuptime _doftime) (Timeline|CardAnimation Play)
            (:Update
              (Variables|/Script/Engine.CameraComponent|SetPostProcessSettings (Variables|/Game/IntBook/TitanicHG/Characters/Player/PlayerCharacter_01/BP_PlayerCharacter_01.BP_PlayerCharacter_01_C|GetCamera (Variables|Default|GetAs%20BP%20Player%20Character%2001)) (Utilities|Struct|MakePostProcessSettings (Math|Float|Lerp (Utilities|Struct|BreakPostProcessSettings (Variables|/Script/Engine.CameraComponent|GetPostProcessSettings (Variables|/Game/IntBook/TitanicHG/Characters/Player/PlayerCharacter_01/BP_PlayerCharacter_01.BP_PlayerCharacter_01_C|GetCamera (Variables|Default|GetAs%20BP%20Player%20Character%2001)))) 1e+01 _doftime)))
              (Transformation|SetRelativeTransform (Variables|Default|GetTestimonialCard) (Math|Transform|Lerp(Transform) _output_get (Math|Transform|MakeTransform "10.000000, 0, 0" "0,90.000000,90.000000") _pickuptime) false false))
            (:StartUIFadeIn
              (bind _returnvalue (UserInterface|CreateWidget "/Game/Developers/thund/InteractiveBook/LogBookTest/Pages/BP_Testimonial_Widget.BP_Testimonial_Widget_C" (Game|GetPlayerController 0)))
              (bind _output_get_2 (Variables|Default|SetTestimonialWidget _returnvalue))
              (UserInterface|Viewport|AddtoViewport _output_get_2 0)
              (bind _newtrack_0 (Timeline|Timeline_2 Play)
                (:Update
                  (Appearance|SetColorandOpacity _output_get_2 (Utilities|Struct|MakeLinearColor 1.0 1.0 1.0 _newtrack_0) :!class /Script/UMG.UserWidget)
                  (Variables|/Game/IntBook/TitanicHG/Characters/Player/PlayerCharacter_01/BP_PlayerCharacter_01.BP_PlayerCharacter_01_C|SetCanRotate _as_bp_player_character_01_4 true)
                  (Variables|/Game/IntBook/TitanicHG/Characters/Player/PlayerCharacter_01/BP_PlayerCharacter_01.BP_PlayerCharacter_01_C|SetCanZoom _as_bp_player_character_01_4 true))
                (:Finished
                  (Variables|Default|SetFullyRendered true))))))))
    (:then_1
      ;[1 1 1] Add to log
      (if (Variables|Default|GetFullyRendered)
        (Variables|/Game/IntBook/TitanicHG/Characters/Player/PlayerCharacter_01/BP_PlayerCharacter_01.BP_PlayerCharacter_01_C|SetCanEnableMouse _as_bp_player_character_01_2 true)
        (Variables|/Game/IntBook/TitanicHG/Characters/Player/PlayerCharacter_01/BP_PlayerCharacter_01.BP_PlayerCharacter_01_C|SetAmInteracting _as_bp_player_character_01_2 false)
        (Variables|/Game/IntBook/TitanicHG/Characters/Player/PlayerCharacter_01/BP_PlayerCharacter_01.BP_PlayerCharacter_01_C|SetCanInteract _as_bp_player_character_01_2 false)
        (Class|InterfaceObjectInteraction|EnableMovement(Message) _as_bp_player_character_01_2)
        (Variables|/Script/Engine.CameraComponent|SetPostProcessSettings (Variables|/Game/IntBook/TitanicHG/Characters/Player/PlayerCharacter_01/BP_PlayerCharacter_01.BP_PlayerCharacter_01_C|GetCamera (Variables|Default|GetAs%20BP%20Player%20Character%2001)) (Utilities|Struct|MakePostProcessSettings 0.0))
        (AddComponent|AddParticleSystemComponent (Game|GetPlayerCharacter 0) false (Variables|Default|GetInitialLocation))
        (bind _asbp_player_character_01 (Utilities|Casting|CastToBP_PlayerCharacter_01 (Game|GetPlayerCharacter 0)))
        (Variables|/Game/IntBook/TitanicHG/Characters/Player/PlayerCharacter_01/BP_PlayerCharacter_01.BP_PlayerCharacter_01_C|SetObject%20Looked%20At _asbp_player_character_01 0)
        (Widget|RemovefromParent (Variables|Default|GetTestimonialWidget))
        (Actor|DestroyActor)))))

(event EventFlipTestimonial
  ;[1 1 1] Flip/Rotate
  (Utilities|FlowControl|Sequence
    (:then_0
      (Utilities|FlowControl|DoOnce false
        (:Completed
          (Variables|Default|SetInitialRotation (Variables|/Script/Engine.SceneComponent|GetRelativeRotation (Variables|Default|GetTestimonialCard))))))
    (:then_1
      (Utilities|FlowControl|FlipFlop
        (:A
          (bind (_direction _time) (Timeline|FlipTimeline Play)
            (:Update
              (switch Utilities|FlowControl|Switch|SwitchonETimelineDirection _direction
                (:Forward
                  (Transformation|SetRelativeRotation (Variables|Default|GetTestimonialCard) (Math|Rotator|Lerp(Rotator) (Variables|Default|GetInitialRotation) (Math|Rotator|CombineRotators (Variables|Default|GetInitialRotation) "0,180.000000, 0") _time) false false))
                (:Backward
                  (Transformation|SetRelativeRotation (Variables|Default|GetTestimonialCard) (Math|Rotator|Lerp(Rotator) (Variables|Default|GetInitialRotation) (Math|Rotator|CombineRotators (Variables|Default|GetInitialRotation) "0,-180.000000, 0") _time) false false))))))
        (:B
          (Timeline|FlipTimeline Reverse))))))

(event EventBeginLookingat
  ;[1 1 1] Set RenderDepth Outline
  (bind _asbp_player_character_01 (Utilities|Casting|CastToBP_PlayerCharacter_01 (Game|GetPlayerCharacter 0)))
  (bind _output_get (Variables|Default|SetAs%20BP%20Player%20Character%2001 _asbp_player_character_01))
  (if (Variables|/Game/IntBook/TitanicHG/Characters/Player/PlayerCharacter_01/BP_PlayerCharacter_01.BP_PlayerCharacter_01_C|GetCanInteract _output_get)
    (Rendering|SetRenderCustomDepth (Variables|Default|GetTestimonialCard) true)
    (Rendering|SetCustomDepthStencilValue (Variables|Default|GetTestimonialCard) 2)
    (Components|Timeline|SetLooping (Variables|Default|GetBlinkColorTimeline) true)
    (Components|Timeline|SetPlayRate (Variables|Default|GetBlinkColorTimeline) (Variables|Default|GetBlinkSpeed))
    (bind (_direction _color _time) (Timeline|BlinkColorTimeline Play)
      (:Update
        (Variables|Default|SetTime _time)
        (Rendering|Material|SetVectorParameterValueonMaterials (Variables|Default|GetTestimonialCard) "BlinkColor" (Math|Conversions|ToVector(LinearColor) _color))
        (Rendering|Material|SetScalarParameterValueonMaterials (Variables|Default|GetTestimonialCard) "BlinkIntensity" (Variables|Default|GetBlinkIntensity))))
    (else
      (Rendering|SetRenderCustomDepth (Variables|Default|GetTestimonialCard) false)
      (Rendering|SetCustomDepthStencilValue (Variables|Default|GetTestimonialCard) 0)
      (Components|Timeline|SetLooping (Variables|Default|GetBlinkColorTimeline) false)
      (Components|Timeline|SetPlayRate (Variables|Default|GetBlinkColorTimeline) (* (Variables|Default|GetBlinkSpeed) 1.0))
      (if (>= (Variables|Default|GetTime) 0.75)
        (Timeline|BlinkColorTimeline Play)
        (else
          (Timeline|BlinkColorTimeline Reverse))))))

(event EventEndLookingat
  ;[1 1 1] Set RenderDepth Outline
  (Rendering|SetRenderCustomDepth (Variables|Default|GetTestimonialCard) false)
  (Rendering|SetCustomDepthStencilValue (Variables|Default|GetTestimonialCard) 0)
  (Components|Timeline|SetLooping (Variables|Default|GetBlinkColorTimeline) false)
  (Components|Timeline|SetPlayRate (Variables|Default|GetBlinkColorTimeline) (* (Variables|Default|GetBlinkSpeed) 1.0))
  (if (>= (Variables|Default|GetTime) 0.75)
    (bind (_direction _color _time) (Timeline|BlinkColorTimeline Play)
      (:Update
        (Variables|Default|SetTime _time)
        (Rendering|Material|SetVectorParameterValueonMaterials (Variables|Default|GetTestimonialCard) "BlinkColor" (Math|Conversions|ToVector(LinearColor) _color))
        (Rendering|Material|SetScalarParameterValueonMaterials (Variables|Default|GetTestimonialCard) "BlinkIntensity" (Variables|Default|GetBlinkIntensity))))
    (else
      (Timeline|BlinkColorTimeline Reverse))))

(fn ConstructionScript)