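; Trigger box Blueprint for an info point that shows a spatial cue widget and lets the player toggle audio playback.
; A custom event receives overlap and info-button states, creating a new cue widget on each overlapping call.
; Pressing the button inside plays or stops the audio, while a non-overlapping call stops it and removes all widgets.
; Tick polls the audio component to keep the playing flag current.
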(event Collision|EventActorBeginOverlap
  (params (OtherActor :type Actor%20Object%20Reference)))

(event EventTick
  (params (DeltaSeconds :type Float%20%28single-precision%29))
  ;[1 1 1] Set "Audio Is Playing" Variable
  (Variables|Default|SetAudio%20Is%20Playing (Audio|Components|Audio|IsPlaying (Variables|Default|GetAudio))))

(event EventPlayerIsOverlappingTrigger
  (params (Player%20Is%20Overlapping%20Trigger%20Volume :type Boolean) (Info%20Interact%20Button%20Pressed :type Boolean))
  (bind _audio (Variables|Default|GetAudio))
  (if Player%20Is%20Overlapping%20Trigger%20Volume
    ;[1 1 1] Play Sound cue when overlapping trigger volume and info interact button is pressed. Sets
    (bind _returnvalue (UserInterface|CreateWidget "/Game/IntBook/TitanicHG/Blueprints/Interactions/BP_Widget_SpatialCue.BP_Widget_SpatialCue_C"))
    (UserInterface|Viewport|AddtoViewport _returnvalue 0)
    (else
      (Viewport|RemoveAllWidgets)))
  (if Player%20Is%20Overlapping%20Trigger%20Volume
    (if Info%20Interact%20Button%20Pressed
      (if (Variables|Default|GetAudio%20Is%20Playing)
        ;[1 1 1] Stop playing audio if player leaves trigger volume or info interact button is pressed again
        (Audio|Components|Audio|Stop (Variables|Default|GetAudio) :!label _label)
        (else
          (Audio|Components|Audio|Play _audio 0.0)
          (Variables|Default|SetAudio%20Is%20Playing (Audio|Components|Audio|IsPlaying _audio)))))
    (else
      (goto _label))))

(fn ConstructionScript)