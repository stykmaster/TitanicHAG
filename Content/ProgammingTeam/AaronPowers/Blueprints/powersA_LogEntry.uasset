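; Log entry actor that builds a Visual, Spacial, Physical or Testimonial page widget filled with its own text and image variables.
; The construction script creates the template chosen by WidgetType, fills it and feeds the PageWidget render target into a dynamic material on Page.
; BeginPlay destroys Page, so that textured page does not persist into play.
; UpdatePage refills the widget, while AudioButtonHighlight only casts to the Visual template.
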(event Custom|AudioButtonHighlight
  (Utilities|Casting|CastToVisual_LogTemplate (Variables|Default|GetwidgetRef)))

(event Custom|UpdatePage
  (CallFunction|SetWidgetVariables))

(event EventBeginPlay
  (Components|DestroyComponent (Variables|Default|GetPage)))

(fn ConstructionScript
  (CallFunction|SpawnWidgets (Variables|LOGTYPE|GetwidgetType))
  (CallFunction|SetWidgetVariables)
  (CallFunction|CreateMaterialInstance))

(fn CreateMaterialInstance
  ;[1 1 1] Set Parameter In Dynamic Material
  (bind _returnvalue (Rendering|Material|CreateDynamicMaterialInstance "/Game/ProgammingTeam/AaronPowers/Materials/TestPageMaterial.testPageMaterial" "None" "None" :!class /Script/Engine.KismetMaterialLibrary))
  (bind _output_get (Variables|Default|SetdynamicMaterial _returnvalue))
  (Rendering|Material|SetTextureParameterValue _output_get "FrontPageRenderTarget" (Class|WidgetComponent|GetRenderTarget (Variables|Default|GetPageWidget)))
  ;[1 1 1] Set Page To Dynamic Material
  (Rendering|Material|SetMaterial (Variables|Default|GetPage) 0 (Variables|Default|GetdynamicMaterial)))

(fn SpawnWidgets
  (params (widgetType :type powersA_pageType%20Enum :default "NewEnumerator0"))
  ;[1 1 1] Set Widget Type To Spawn
  (switch Utilities|FlowControl|Switch|SwitchonpowersA_pageType widgetType
    (:NewEnumerator0
      (Variables|Default|Setwidget "/Game/AntonioSmith/Visual_LogTemplate.Visual_LogTemplate_C"))
    (:NewEnumerator1
      (Variables|Default|Setwidget "/Game/Developers/tyler/Collections/Spacial_LogTemplate.Spacial_LogTemplate_C"))
    (:NewEnumerator2
      (Variables|Default|Setwidget "/Game/Developers/tyler/Collections/Physical_LogTemplate.Physical_LogTemplate_C"))
    (:NewEnumerator3
      (Variables|Default|Setwidget "/Game/AntonioSmith/Testimonial_LogTemplate.Testimonial_LogTemplate_C")))
  ;[1 1 1] Spawn Widget, Set to Ref, and Set Widget Component To Render Widget
  (bind _returnvalue (UserInterface|CreateWidget (Variables|Default|Getwidget)))
  (bind _output_get (Variables|Default|SetwidgetRef _returnvalue))
  (UserInterface|SetWidget (Variables|Default|GetPageWidget) _output_get)
  (return))

(fn SetWidgetVariables
  (bind _widgetref (Variables|Default|GetwidgetRef))
  ;[1 1 1] Set Front Widget Variables Based On Widget Type
  (switch Utilities|FlowControl|Switch|SwitchonpowersA_pageType (Variables|LOGTYPE|GetwidgetType)
    (:NewEnumerator0
      (CallFunction|SetVisualPageWidgetVariables _widgetref))
    (:NewEnumerator1
      (CallFunction|SetSpacialPageWidgetVariables _widgetref))
    (:NewEnumerator2
      (CallFunction|SetPhysicalPageWidgetVariables _widgetref))
    (:NewEnumerator3
      (CallFunction|SetTestimonialPageWidgetVariables _widgetref)))
  (return))

(fn SetVisualPageWidgetVariables
  (params (visualWidget :type User%20Widget%20Object%20Reference))
  (bind _asvisual_log_template (Utilities|Casting|CastToVisual_LogTemplate visualWidget))
  ;[1 1 1] Set Visual Log Variables
  (Rendering|Components|TextRender|SetText (Variables|/Game/AntonioSmith/Visual_LogTemplate.Visual_LogTemplate_C|GetDeckNameInfo _asvisual_log_template) (Variables|LOGSETTINGS|GetdeckNameInfo))
  (Rendering|Components|TextRender|SetText (Variables|/Game/AntonioSmith/Visual_LogTemplate.Visual_LogTemplate_C|GetPageTitle _asvisual_log_template) (Variables|LOGSETTINGS|GetpageTitle))
  (Rendering|Components|TextRender|SetText (Variables|/Game/AntonioSmith/Visual_LogTemplate.Visual_LogTemplate_C|GetPhotographerInfo _asvisual_log_template) (Variables|LOGSETTINGS|VISUALLogSettings|GetphotographerInfo))
  (Rendering|Components|TextRender|SetText (Variables|/Game/AntonioSmith/Visual_LogTemplate.Visual_LogTemplate_C|GetTakenInfo _asvisual_log_template) (Variables|LOGSETTINGS|VISUALLogSettings|GettakenInfo))
  (Appearance|SetBrushfromTexture (Variables|/Game/AntonioSmith/Visual_LogTemplate.Visual_LogTemplate_C|GetVisualImage _asvisual_log_template) (Variables|LOGSETTINGS|VISUALLogSettings|GetvisualImage) false))

(fn SetSpacialPageWidgetVariables
  (params (spacialWidget :type User%20Widget%20Object%20Reference))
  (bind _asspacial_log_template (Utilities|Casting|CastToSpacial_LogTemplate spacialWidget))
  ;[1 1 1] Set Spacial Log Variables
  (Rendering|Components|TextRender|SetText (Variables|/Game/Developers/tyler/Collections/Spacial_LogTemplate.Spacial_LogTemplate_C|GetDeckNameInfo _asspacial_log_template) (Variables|LOGSETTINGS|GetdeckNameInfo))
  (Rendering|Components|TextRender|SetText (Variables|/Game/Developers/tyler/Collections/Spacial_LogTemplate.Spacial_LogTemplate_C|GetPageTitle _asspacial_log_template) (Variables|LOGSETTINGS|GetpageTitle))
  (Rendering|Components|TextRender|SetText (Variables|/Game/Developers/tyler/Collections/Spacial_LogTemplate.Spacial_LogTemplate_C|GetMainUseInfo _asspacial_log_template) (Variables|LOGSETTINGS|SPACIALLogSettings|GetmainUseInfo))
  (Rendering|Components|TextRender|SetText (Variables|/Game/Developers/tyler/Collections/Spacial_LogTemplate.Spacial_LogTemplate_C|GetAccessInfo _asspacial_log_template) (Variables|LOGSETTINGS|SPACIALLogSettings|GetaccessInfo))
  (Rendering|Components|TextRender|SetText (Variables|/Game/Developers/tyler/Collections/Spacial_LogTemplate.Spacial_LogTemplate_C|GetFlooringInfo _asspacial_log_template) (Variables|LOGSETTINGS|SPACIALLogSettings|GetflooringInfo))
  (Appearance|SetBrushfromTexture (Variables|/Game/Developers/tyler/Collections/Spacial_LogTemplate.Spacial_LogTemplate_C|GetSpacialImage _asspacial_log_template) (Variables|LOGSETTINGS|SPACIALLogSettings|GetspacialImage) false))

(fn SetPhysicalPageWidgetVariables
  (params (physicalWidget :type User%20Widget%20Object%20Reference))
  (bind _asphysical_log_template (Utilities|Casting|CastToPhysical_LogTemplate physicalWidget))
  ;[1 1 1] Set Physical Log Variables
  (Rendering|Components|TextRender|SetText (Variables|/Game/Developers/tyler/Collections/Physical_LogTemplate.Physical_LogTemplate_C|GetDeckNameInfo _asphysical_log_template) (Variables|LOGSETTINGS|GetdeckNameInfo))
  (Rendering|Components|TextRender|SetText (Variables|/Game/Developers/tyler/Collections/Physical_LogTemplate.Physical_LogTemplate_C|GetPageTitle _asphysical_log_template) (Variables|LOGSETTINGS|GetpageTitle))
  (Rendering|Components|TextRender|SetText (Variables|/Game/Developers/tyler/Collections/Physical_LogTemplate.Physical_LogTemplate_C|GetManufacturerInfo _asphysical_log_template) (Variables|LOGSETTINGS|PHYSICALLogSettings|GetmanufacturerInfo))
  (Rendering|Components|TextRender|SetText (Variables|/Game/Developers/tyler/Collections/Physical_LogTemplate.Physical_LogTemplate_C|GetMaterialInfo _asphysical_log_template) (Variables|LOGSETTINGS|PHYSICALLogSettings|GetmaterialsInfo))
  (Rendering|Components|TextRender|SetText (Variables|/Game/Developers/tyler/Collections/Physical_LogTemplate.Physical_LogTemplate_C|GetDimensionsInfo _asphysical_log_template) (Variables|LOGSETTINGS|PHYSICALLogSettings|GetdimensionsInfo))
  (Rendering|Components|TextRender|SetText (Variables|/Game/Developers/tyler/Collections/Physical_LogTemplate.Physical_LogTemplate_C|GetTypeInfo _asphysical_log_template) (Variables|LOGSETTINGS|PHYSICALLogSettings|GettypeInfo))
  (Appearance|SetBrushfromTexture (Variables|/Game/Developers/tyler/Collections/Physical_LogTemplate.Physical_LogTemplate_C|GetPhysicalImage _asphysical_log_template) (Variables|LOGSETTINGS|PHYSICALLogSettings|GetphysicalImage) false))

(fn SetTestimonialPageWidgetVariables
  (params (testimonialWidget :type User%20Widget%20Object%20Reference))
  (bind _astestimonial_log_template (Utilities|Casting|CastToTestimonial_LogTemplate testimonialWidget))
  ;[1 1 1] Set Testimonial Log Variables
  (Rendering|Components|TextRender|SetText (Variables|/Game/AntonioSmith/Testimonial_LogTemplate.Testimonial_LogTemplate_C|GetDeckNameInfo _astestimonial_log_template) (Variables|LOGSETTINGS|GetdeckNameInfo))
  (Rendering|Components|TextRender|SetText (Variables|/Game/AntonioSmith/Testimonial_LogTemplate.Testimonial_LogTemplate_C|GetpageTitle _astestimonial_log_template) (Variables|LOGSETTINGS|GetpageTitle))
  (Rendering|Components|TextRender|SetText (Variables|/Game/AntonioSmith/Testimonial_LogTemplate.Testimonial_LogTemplate_C|GetAgeInfo _astestimonial_log_template) (Variables|LOGSETTINGS|TESTIMONIALLogSettings|GetageInfo))
  (Rendering|Components|TextRender|SetText (Variables|/Game/AntonioSmith/Testimonial_LogTemplate.Testimonial_LogTemplate_C|GetClassInfo _astestimonial_log_template) (Variables|LOGSETTINGS|TESTIMONIALLogSettings|GetclassInfo))
  (Rendering|Components|TextRender|SetText (Variables|/Game/AntonioSmith/Testimonial_LogTemplate.Testimonial_LogTemplate_C|GetBirthplaceInfo _astestimonial_log_template) (Variables|LOGSETTINGS|TESTIMONIALLogSettings|GetbirthplaceInfo))
  (Rendering|Components|TextRender|SetText (Variables|/Game/AntonioSmith/Testimonial_LogTemplate.Testimonial_LogTemplate_C|GetDestinationInfo _astestimonial_log_template) (Variables|LOGSETTINGS|TESTIMONIALLogSettings|GetdestinationInfo))
  (Appearance|SetBrushfromTexture (Variables|/Game/AntonioSmith/Testimonial_LogTemplate.Testimonial_LogTemplate_C|GetTestimonialImage _astestimonial_log_template) (Variables|LOGSETTINGS|TESTIMONIALLogSettings|GettestimonialImage) false))