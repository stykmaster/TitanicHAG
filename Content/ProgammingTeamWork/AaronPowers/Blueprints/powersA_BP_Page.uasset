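; Page actor that shows a front and back log entry on a single page mesh.
; It spawns log entry actors from two classes, then feeds their widget render targets into a dynamic material on the Page mesh as texture parameters.
; BeginPlay waits a brief delay before building the material.
; ChangePage destroys and respawns the entries, while UpdatePage refreshes them and recreates the material.
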(event Custom|UpdatePage
  (Default|UpdatePage (Variables|Default|GetfrontLogRef))
  (Default|UpdatePage (Variables|Default|GetbackLogRef))
  (CallFunction|CreateMaterialInstance))

(event Custom|ChangePage
  (CallFunction|ClearOldWidgets)
  (CallFunction|SpawnWidgetReferences)
  (Utilities|FlowControl|Delay 0.017)
  (CallFunction|CreateMaterialInstance))

(event EventBeginPlay
  (CallFunction|SpawnWidgetReferences)
  (Utilities|FlowControl|Delay 0.017)
  (CallFunction|CreateMaterialInstance))

(fn ConstructionScript)

(fn CreateMaterialInstance
  (bind _frontlogref (Variables|Default|GetfrontLogRef))
  (bind _backlogref (Variables|Default|GetbackLogRef))
  (bind _returnvalue (Rendering|Material|CreateDynamicMaterialInstance "/Game/ProgammingTeamWork/AaronPowers/Materials/testPageMaterial.testPageMaterial" "None" "None" :!class /Script/Engine.KismetMaterialLibrary))
  (Variables|Default|SetdynamicMaterial _returnvalue)
  ;[1 1 1] Assign Render Textures To Dynamic Material Parameters
  (Utilities|IsValid _frontlogref
    (:Is%20Valid
      (Rendering|Material|SetTextureParameterValue (Variables|Default|GetdynamicMaterial) "FrontPageRenderTarget" (Class|WidgetComponent|GetRenderTarget (Variables|/Game/ProgammingTeamWork/AaronPowers/Blueprints/powersA_LogEntry.powersA_LogEntry_C|GetPageWidget _frontlogref))))
    (:Is%20Not%20Valid
      _))
  (Utilities|IsValid _backlogref
    (:Is%20Valid
      (Rendering|Material|SetTextureParameterValue (Variables|Default|GetdynamicMaterial) "BackPageRenderTarget" (Class|WidgetComponent|GetRenderTarget (Variables|/Game/ProgammingTeamWork/AaronPowers/Blueprints/powersA_LogEntry.powersA_LogEntry_C|GetPageWidget _backlogref))))
    (:Is%20Not%20Valid
      _))
  ;[1 1 1] Set Material To Page
  (Rendering|Material|SetMaterial (Variables|Default|GetPage) 0 (Variables|Default|GetdynamicMaterial)))

(fn UpdateMaterialInstance
  (bind _frontlogref (Variables|Default|GetfrontLogRef))
  (bind _backlogref (Variables|Default|GetbackLogRef))
  ;[1 1 1] Assign Render Textures To Dynamic Material Parameters
  (Utilities|IsValid _frontlogref
    (:Is%20Valid
      (Rendering|Material|SetTextureParameterValue (Variables|Default|GetdynamicMaterial) "FrontPageRenderTarget" (Class|WidgetComponent|GetRenderTarget (Variables|/Game/ProgammingTeamWork/AaronPowers/Blueprints/powersA_LogEntry.powersA_LogEntry_C|GetPageWidget _frontlogref))))
    (:Is%20Not%20Valid
      _))
  (Utilities|IsValid _backlogref
    (:Is%20Valid
      (Rendering|Material|SetTextureParameterValue (Variables|Default|GetdynamicMaterial) "BackPageRenderTarget" (Class|WidgetComponent|GetRenderTarget (Variables|/Game/ProgammingTeamWork/AaronPowers/Blueprints/powersA_LogEntry.powersA_LogEntry_C|GetPageWidget _backlogref))))
    (:Is%20Not%20Valid
      _))
  ;[1 1 1] Set Material To Page
  (Rendering|Material|SetMaterial (Variables|Default|GetPage) 0 (Variables|Default|GetdynamicMaterial)))

(fn SpawnWidgetReferences
  (bind _frontlogentry (Variables|Default|GetfrontLogEntry))
  (bind _backlogentry (Variables|Default|GetbackLogEntry))
  (bind _defaultsceneroot (Variables|Default|GetDefaultSceneRoot))
  (bind _returnvalue (Transformation|GetWorldTransform _defaultsceneroot))
  ;[1 1 1] Spawn Front Log Entry
  (if (Utilities|IsValidClass _frontlogentry)
    (bind _returnvalue_2 (Game|SpawnActorfromClass _frontlogentry _returnvalue "Undefined" 0 0))
    (Variables|Default|SetfrontLogRef _returnvalue_2)
    ;[1 1 1] Spawn Back Log Entry
    (if (Utilities|IsValidClass _backlogentry)
      (bind _returnvalue_3 (Game|SpawnActorfromClass _backlogentry _returnvalue "Undefined" 0 0))
      (Variables|Default|SetbackLogRef _returnvalue_3))))

(fn ClearOldWidgets
  (Actor|DestroyActor (Variables|Default|GetfrontLogRef)))