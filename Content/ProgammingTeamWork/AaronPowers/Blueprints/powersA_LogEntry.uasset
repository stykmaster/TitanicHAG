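; Log entry page actor that shows one of four log types (visual, spacial, physical, testimonial) with text, image and page number.
; The construction script spawns the matching template widget, fills it from the entry's variables and feeds the widget's render target into the page's dynamic material.
; Narration and information button events swap icon brushes and tints, then request a widget redraw.
; BeginPlay destroys the Page component and requests a render update.
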(event Custom|NarrationButtonUnhover
  (BUTTONFUNCTIONS|ButtonUnhover (Variables|Default|GetnarrationButton) true)
  (UserInterface|RequestRenderUpdate (Variables|Default|GetPageWidget)))

(event Custom|UpdatePage
  (SETWIDGET|SetWidgetVariables)
  (UserInterface|RequestRenderUpdate (Variables|Default|GetPageWidget)))

(event Custom|NarrationButtonClick
  (BUTTONFUNCTIONS|ButtonClick (Variables|Default|GetnarrationButton) true)
  (UserInterface|RequestRenderUpdate (Variables|Default|GetPageWidget)))

(event Custom|InformationButtonClick
  (BUTTONFUNCTIONS|ButtonClick (Variables|Default|GetInformation%20Button) false)
  (UserInterface|RequestRenderUpdate (Variables|Default|GetPageWidget)))

(event Custom|InformationButtonUnhover
  (BUTTONFUNCTIONS|ButtonUnhover (Variables|Default|GetInformation%20Button) false)
  (UserInterface|RequestRenderUpdate (Variables|Default|GetPageWidget)))

(event Custom|InformationButtonHover
  (BUTTONFUNCTIONS|ButtonHover (Variables|Default|GetInformation%20Button) false)
  (UserInterface|RequestRenderUpdate (Variables|Default|GetPageWidget)))

(event Custom|NarrationButtonHover
  (BUTTONFUNCTIONS|ButtonHover (Variables|Default|GetnarrationButton) true)
  (UserInterface|RequestRenderUpdate (Variables|Default|GetPageWidget)))

(event EventBeginPlay
  (Components|DestroyComponent (Variables|Default|GetPage))
  (UserInterface|RequestRenderUpdate (Variables|Default|GetPageWidget)))

(fn ConstructionScript
  (CallFunction|SpawnWidgets (Variables|LOGTYPE|GetwidgetType))
  (SETWIDGET|SetWidgetVariables)
  (CallFunction|CreateMaterialInstance))

(fn CreateMaterialInstance
  ;[1 1 1] Set Parameter In Dynamic Material
  (bind _returnvalue (Rendering|Material|CreateDynamicMaterialInstance "/Game/ProgammingTeamWork/AaronPowers/Materials/testPageMaterial.testPageMaterial" "None" "None" :!class /Script/Engine.KismetMaterialLibrary))
  (bind _output_get (Variables|Default|SetdynamicMaterial _returnvalue))
  (Rendering|Material|SetTextureParameterValue _output_get "FrontPageRenderTarget" (Class|WidgetComponent|GetRenderTarget (Variables|Default|GetPageWidget)))
  ;[1 1 1] Set Page To Dynamic Material
  (Rendering|Material|SetMaterial (Variables|Default|GetPage) 0 (Variables|Default|GetdynamicMaterial)))

(fn SpawnWidgets
  (params (widgetType :type powersA_pageType%20Enum :default "NewEnumerator0"))
  ;[1 1 1] Set Widget Type To Spawn
  (switch Utilities|FlowControl|Switch|SwitchonpowersA_pageType widgetType
    (:NewEnumerator0
      (Variables|Default|Setwidget "/Game/Developers/wapas/Visual_LogTemplate.Visual_LogTemplate_C"))
    (:NewEnumerator1
      (Variables|Default|Setwidget "/Game/Developers/tyler/Collections/Spacial_LogTemplate.Spacial_LogTemplate_C"))
    (:NewEnumerator2
      (Variables|Default|Setwidget "/Game/Developers/tyler/Collections/Physical_LogTemplate.Physical_LogTemplate_C"))
    (:NewEnumerator3
      (Variables|Default|Setwidget "/Game/Developers/wapas/Testimonial_LogTemplate.Testimonial_LogTemplate_C")))
  ;[1 1 1] Spawn Widget, Set to Ref, and Set Widget Component To Render Widget
  (bind _returnvalue (UserInterface|CreateWidget (Variables|Default|Getwidget)))
  (bind _output_get (Variables|Default|SetwidgetRef _returnvalue))
  (UserInterface|SetWidget (Variables|Default|GetPageWidget) _output_get)
  (return))

(fn SetWidgetVariables
  (bind _widgetref (Variables|Default|GetwidgetRef))
  ;[1 1 1] Set Front Widget Variables Based On Widget Type
  (switch Utilities|FlowControl|Switch|SwitchonpowersA_pageType (Variables|LOGTYPE|GetwidgetType)
    (:NewEnumerator0
      (SETWIDGET|SetVisualPageWidgetVariables _widgetref))
    (:NewEnumerator1
      (SETWIDGET|SetSpacialPageWidgetVariables _widgetref))
    (:NewEnumerator2
      (SETWIDGET|SetPhysicalPageWidgetVariables _widgetref))
    (:NewEnumerator3
      (SETWIDGET|SetTestimonialPageWidgetVariables _widgetref)))
  (return))

(fn SetVisualPageWidgetVariables
  (params (visualWidget :type User%20Widget%20Object%20Reference))
  (bind _asvisual_log_template (Utilities|Casting|CastToVisual_LogTemplate visualWidget))
  ;[1 1 1] Set Visual Log Variables
  (Rendering|Components|TextRender|SetText (Variables|/Game/Developers/wapas/Visual_LogTemplate.Visual_LogTemplate_C|GetDeckNameInfo _asvisual_log_template) (Variables|LOGSETTINGS|GetdeckNameInfo))
  (Rendering|Components|TextRender|SetText (Variables|/Game/Developers/wapas/Visual_LogTemplate.Visual_LogTemplate_C|GetPageTitle _asvisual_log_template) (Variables|LOGSETTINGS|GetpageTitle))
  (Rendering|Components|TextRender|SetText (Variables|/Game/Developers/wapas/Visual_LogTemplate.Visual_LogTemplate_C|GetPhotographerInfo _asvisual_log_template) (Variables|LOGSETTINGS|GetphotographerInfo))
  (Rendering|Components|TextRender|SetText (Variables|/Game/Developers/wapas/Visual_LogTemplate.Visual_LogTemplate_C|GetTakenInfo _asvisual_log_template) (Variables|LOGSETTINGS|GettakenInfo))
  (Appearance|SetBrushfromTexture (Variables|/Game/Developers/wapas/Visual_LogTemplate.Visual_LogTemplate_C|GetVisualImage _asvisual_log_template) (Variables|LOGSETTINGS|GetvisualImage) false)
  ;[1 1 1] Set Button Variables
  (Variables|Default|SetnarrationButton (Variables|/Game/Developers/wapas/Visual_LogTemplate.Visual_LogTemplate_C|GetNarrationButton _asvisual_log_template))
  (Variables|Default|SetInformation%20Button (Variables|/Game/Developers/wapas/Visual_LogTemplate.Visual_LogTemplate_C|GetInformationButton _asvisual_log_template))
  ;[1 1 1] Set Text
  (Rendering|Components|TextRender|SetText (Variables|/Game/Developers/wapas/Visual_LogTemplate.Visual_LogTemplate_C|GetPageNumber _asvisual_log_template) (Variables|Default|GetpageNumberVariable)))

(fn SetSpacialPageWidgetVariables
  (params (spacialWidget :type User%20Widget%20Object%20Reference))
  (bind _asspacial_log_template (Utilities|Casting|CastToSpacial_LogTemplate spacialWidget))
  ;[1 1 1] Set Spacial Log Variables
  (Rendering|Components|TextRender|SetText (Variables|/Game/Developers/tyler/Collections/Spacial_LogTemplate.Spacial_LogTemplate_C|GetDeckNameInfo _asspacial_log_template) (Variables|LOGSETTINGS|GetdeckNameInfo))
  (Rendering|Components|TextRender|SetText (Variables|/Game/Developers/tyler/Collections/Spacial_LogTemplate.Spacial_LogTemplate_C|GetPageTitle _asspacial_log_template) (Variables|LOGSETTINGS|GetpageTitle))
  (Rendering|Components|TextRender|SetText (Variables|/Game/Developers/tyler/Collections/Spacial_LogTemplate.Spacial_LogTemplate_C|GetMainUseInfo _asspacial_log_template) (Variables|LOGSETTINGS|GetmainUseInfo))
  (Rendering|Components|TextRender|SetText (Variables|/Game/Developers/tyler/Collections/Spacial_LogTemplate.Spacial_LogTemplate_C|GetAccessInfo _asspacial_log_template) (Variables|LOGSETTINGS|GetaccessInfo))
  (Rendering|Components|TextRender|SetText (Variables|/Game/Developers/tyler/Collections/Spacial_LogTemplate.Spacial_LogTemplate_C|GetFlooringInfo _asspacial_log_template) (Variables|LOGSETTINGS|GetflooringInfo))
  (Appearance|SetBrushfromTexture (Variables|/Game/Developers/tyler/Collections/Spacial_LogTemplate.Spacial_LogTemplate_C|GetSpacialImage _asspacial_log_template) (Variables|LOGSETTINGS|GetspacialImage) false)
  ;[1 1 1] Set Button Variables
  (Variables|Default|SetnarrationButton (Variables|/Game/Developers/tyler/Collections/Spacial_LogTemplate.Spacial_LogTemplate_C|GetNarrationButton _asspacial_log_template))
  (Variables|Default|SetInformation%20Button (Variables|/Game/Developers/tyler/Collections/Spacial_LogTemplate.Spacial_LogTemplate_C|GetInformationButton _asspacial_log_template))
  ;[1 1 1] Set Text
  (Rendering|Components|TextRender|SetText (Variables|/Game/Developers/tyler/Collections/Spacial_LogTemplate.Spacial_LogTemplate_C|GetPageNumber _asspacial_log_template) (Variables|Default|GetpageNumberVariable)))

(fn SetPhysicalPageWidgetVariables
  (params (physicalWidget :type User%20Widget%20Object%20Reference))
  (bind _asphysical_log_template (Utilities|Casting|CastToPhysical_LogTemplate physicalWidget))
  ;[1 1 1] Set Physical Log Variables
  (Rendering|Components|TextRender|SetText (Variables|/Game/Developers/tyler/Collections/Physical_LogTemplate.Physical_LogTemplate_C|GetDeckNameInfo _asphysical_log_template) (Variables|LOGSETTINGS|GetdeckNameInfo))
  (Rendering|Components|TextRender|SetText (Variables|/Game/Developers/tyler/Collections/Physical_LogTemplate.Physical_LogTemplate_C|GetPageTitle _asphysical_log_template) (Variables|LOGSETTINGS|GetpageTitle))
  (Rendering|Components|TextRender|SetText (Variables|/Game/Developers/tyler/Collections/Physical_LogTemplate.Physical_LogTemplate_C|GetManufacturerInfo _asphysical_log_template) (Variables|LOGSETTINGS|GetmanufacturerInfo))
  (Rendering|Components|TextRender|SetText (Variables|/Game/Developers/tyler/Collections/Physical_LogTemplate.Physical_LogTemplate_C|GetMaterialInfo _asphysical_log_template) (Variables|LOGSETTINGS|GetmaterialsInfo))
  (Rendering|Components|TextRender|SetText (Variables|/Game/Developers/tyler/Collections/Physical_LogTemplate.Physical_LogTemplate_C|GetDimensionsInfo _asphysical_log_template) (Variables|LOGSETTINGS|GetdimensionsInfo))
  (Rendering|Components|TextRender|SetText (Variables|/Game/Developers/tyler/Collections/Physical_LogTemplate.Physical_LogTemplate_C|GetTypeInfo _asphysical_log_template) (Variables|LOGSETTINGS|GettypeInfo))
  (Appearance|SetBrushfromTexture (Variables|/Game/Developers/tyler/Collections/Physical_LogTemplate.Physical_LogTemplate_C|GetPhysicalImage _asphysical_log_template) (Variables|LOGSETTINGS|GetphysicalImage) false)
  ;[1 1 1] Set Button Variables
  (Variables|Default|SetnarrationButton (Variables|/Game/Developers/tyler/Collections/Physical_LogTemplate.Physical_LogTemplate_C|GetNarrationButton _asphysical_log_template))
  (Variables|Default|SetInformation%20Button (Variables|/Game/Developers/tyler/Collections/Physical_LogTemplate.Physical_LogTemplate_C|GetInformationButton _asphysical_log_template))
  ;[1 1 1] Set Text
  (Rendering|Components|TextRender|SetText (Variables|/Game/Developers/tyler/Collections/Physical_LogTemplate.Physical_LogTemplate_C|GetPageNumber _asphysical_log_template) (Variables|Default|GetpageNumberVariable)))

(fn SetTestimonialPageWidgetVariables
  (params (testimonialWidget :type User%20Widget%20Object%20Reference))
  (bind _astestimonial_log_template (Utilities|Casting|CastToTestimonial_LogTemplate testimonialWidget))
  ;[1 1 1] Set Testimonial Log Variables
  (Rendering|Components|TextRender|SetText (Variables|/Game/Developers/wapas/Testimonial_LogTemplate.Testimonial_LogTemplate_C|GetDeckNameInfo _astestimonial_log_template) (Variables|LOGSETTINGS|GetdeckNameInfo))
  (Rendering|Components|TextRender|SetText (Variables|/Game/Developers/wapas/Testimonial_LogTemplate.Testimonial_LogTemplate_C|GetpageTitle _astestimonial_log_template) (Variables|LOGSETTINGS|GetpageTitle))
  (Rendering|Components|TextRender|SetText (Variables|/Game/Developers/wapas/Testimonial_LogTemplate.Testimonial_LogTemplate_C|GetAgeInfo _astestimonial_log_template) (Variables|LOGSETTINGS|GetageInfo))
  (Rendering|Components|TextRender|SetText (Variables|/Game/Developers/wapas/Testimonial_LogTemplate.Testimonial_LogTemplate_C|GetClassInfo _astestimonial_log_template) (Variables|LOGSETTINGS|GetclassInfo))
  (Rendering|Components|TextRender|SetText (Variables|/Game/Developers/wapas/Testimonial_LogTemplate.Testimonial_LogTemplate_C|GetBirthplaceInfo _astestimonial_log_template) (Variables|LOGSETTINGS|GetbirthplaceInfo))
  (Rendering|Components|TextRender|SetText (Variables|/Game/Developers/wapas/Testimonial_LogTemplate.Testimonial_LogTemplate_C|GetDestinationInfo _astestimonial_log_template) (Variables|LOGSETTINGS|GetdestinationInfo))
  (Appearance|SetBrushfromTexture (Variables|/Game/Developers/wapas/Testimonial_LogTemplate.Testimonial_LogTemplate_C|GetTestimonialImage _astestimonial_log_template) (Variables|LOGSETTINGS|GettestimonialImage) false)
  ;[1 1 1] Set Button Variables
  (Variables|Default|SetnarrationButton (Variables|/Game/Developers/wapas/Testimonial_LogTemplate.Testimonial_LogTemplate_C|GetNarrationButton _astestimonial_log_template))
  (Variables|Default|SetInformation%20Button (Variables|/Game/Developers/wapas/Testimonial_LogTemplate.Testimonial_LogTemplate_C|GetInformationButton _astestimonial_log_template))
  ;[1 1 1] Set Text
  (Rendering|Components|TextRender|SetText (Variables|/Game/Developers/wapas/Testimonial_LogTemplate.Testimonial_LogTemplate_C|GetPageNumber _astestimonial_log_template) (Variables|Default|GetpageNumberVariable)))

(fn ButtonHover
  (params (buttonImage :type Image%20Object%20Reference) (isNarration :type Boolean))
  (if isNarration
    (Appearance|SetBrushfromTexture buttonImage "/Game/Developers/tyler/Collections/Log_Book_Assets/Log_Book_Assets/icons/white/play_icon.play_icon" false)
    (Appearance|SetColorandOpacity buttonImage "(R=1.000000,G=1.000000,B=1.000000,A=1.000000)" :!class /Script/UMG.Image)
    (else
      (Appearance|SetBrushfromTexture buttonImage "/Game/Developers/tyler/Collections/Log_Book_Assets/Log_Book_Assets/icons/white/source_icon.source_icon" false)
      (Appearance|SetColorandOpacity buttonImage "(R=1.000000,G=1.000000,B=1.000000,A=1.000000)" :!class /Script/UMG.Image))))

(fn ButtonUnhover
  (params (buttonImage :type Image%20Object%20Reference) (isNarration :type Boolean))
  (if isNarration
    (Appearance|SetBrushfromTexture buttonImage "/Game/Developers/tyler/Collections/Log_Book_Assets/Log_Book_Assets/icons/color/play_icon.play_icon" false)
    (Appearance|SetColorandOpacity buttonImage "(R=1.000000,G=1.000000,B=1.000000,A=1.000000)" :!class /Script/UMG.Image)
    (else
      (Appearance|SetBrushfromTexture buttonImage "/Game/Developers/tyler/Collections/Log_Book_Assets/Log_Book_Assets/icons/color/source_icon.source_icon" false)
      (Appearance|SetColorandOpacity buttonImage "(R=1.000000,G=1.000000,B=1.000000,A=1.000000)" :!class /Script/UMG.Image))))

(fn ButtonClick
  (params (buttonImage :type Image%20Object%20Reference) (isNarration :type Boolean))
  (if isNarration
    (Appearance|SetBrushfromTexture buttonImage "/Game/Developers/tyler/Collections/Log_Book_Assets/Log_Book_Assets/icons/color/play_icon.play_icon" false)
    (Appearance|SetColorandOpacity buttonImage "(R=0.500000,G=0.500000,B=0.500000,A=1.000000)" :!class /Script/UMG.Image)
    (else
      (Appearance|SetBrushfromTexture buttonImage "/Game/Developers/tyler/Collections/Log_Book_Assets/Log_Book_Assets/icons/color/source_icon.source_icon" false)
      (Appearance|SetColorandOpacity buttonImage "(R=0.500000,G=0.500000,B=0.500000,A=1.000000)" :!class /Script/UMG.Image))))

(fn SetPageNumberText
  (bind _pagenumbervariable (Variables|Default|GetpageNumberVariable))
  (bind _widgetref (Variables|Default|GetwidgetRef))
  (switch Utilities|FlowControl|Switch|SwitchonpowersA_pageType (Variables|LOGTYPE|GetwidgetType)
    (:NewEnumerator0
      (bind _asvisual_log_template (Utilities|Casting|CastToVisual_LogTemplate _widgetref))
      (Rendering|Components|TextRender|SetText (Variables|/Game/Developers/wapas/Visual_LogTemplate.Visual_LogTemplate_C|GetPageNumber _asvisual_log_template) _pagenumbervariable))
    (:NewEnumerator1
      (bind _asspacial_log_template (Utilities|Casting|CastToSpacial_LogTemplate _widgetref))
      (Rendering|Components|TextRender|SetText (Variables|/Game/Developers/tyler/Collections/Spacial_LogTemplate.Spacial_LogTemplate_C|GetPageNumber _asspacial_log_template) _pagenumbervariable))
    (:NewEnumerator2
      (bind _asphysical_log_template (Utilities|Casting|CastToPhysical_LogTemplate _widgetref))
      (Rendering|Components|TextRender|SetText (Variables|/Game/Developers/tyler/Collections/Physical_LogTemplate.Physical_LogTemplate_C|GetPageNumber _asphysical_log_template) _pagenumbervariable))
    (:NewEnumerator3
      (bind _astestimonial_log_template (Utilities|Casting|CastToTestimonial_LogTemplate _widgetref))
      (Rendering|Components|TextRender|SetText (Variables|/Game/Developers/wapas/Testimonial_LogTemplate.Testimonial_LogTemplate_C|GetPageNumber _astestimonial_log_template) _pagenumbervariable))))